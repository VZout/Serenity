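; Enemy ship AI pawn that turns toward, chases and fires at player 0.
; Tick gates smoothed rotation on a sight check, though that trace starts and ends at the player's location.
; Within range, it advances until too close, while a Delay throttles Attack0 to roughly once a second.
; Attack0 spawns B_Bullet at every mesh socket, leaving the "Weapon0" prefix filter unwired; Attack1 is an empty stub.
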(event `self.ReceiveBeginPlay`)

(event `self.ReceiveActorBeginOverlap`
  (params (OtherActor :type "Actor Object Reference")))

(event `self.ReceiveTick`
  (params (DeltaSeconds :type "Float (single-precision)"))
  (bind _haslineofsight (`self.EnemyHasLineOfSight`))
  (if _haslineofsight
    (`self.RotateTowardsPlayer` 10.0 DeltaSeconds)
    (bind _isindistance (`self.PlayerIsInDistance`))
    (if _isindistance
      (`|ExecutionSequence`
        (:`then_0`
          (`KismetSystemLibrary.Delay` 1.0)
          (`self.Attack0`))
        (:`then_1`
          (bind _isindistance_2 (`self.PlayerIsToClose`))
          (if (not _isindistance_2)
            (`self.MoveTowardsPlayer`)))
        (:`then_2`
          (`self.Attack1`))))))

(fn `Attack0`
  (for _array_element (`SceneComponent.GetAllSocketNames` (`self.StaticMesh`))
    (if true
      (`|SpawnActorFromClass` "/Game/B_Bullet.B_Bullet_C" (`SceneComponent.GetSocketTransform` (`self.StaticMesh`) _array_element "RTS_World") "Undefined" "OverrideRootScale"))))

(fn `Attack1`)

(fn `EnemyHasLineOfSight`
  (returns (hasLineOfSight :type Boolean))
  (bind _returnvalue (`GameplayStatics.GetPlayerPawn` 0))
  (bind (_outhit _returnvalue_2) (`KismetSystemLibrary.LineTraceSingle` (`self.K2_GetActorLocation` _returnvalue) (`self.K2_GetActorLocation` _returnvalue) "TraceTypeQuery1" true (`|MakeArray` _returnvalue :!type "Actor Object Reference")))
  (return (not _returnvalue_2)))

(fn `GetDistanceBetweenPlayer`
  (returns (Distance :type "Float (double-precision)"))
  (return (`KismetMathLibrary.VSize` (- (`self.K2_GetActorLocation`) (`self.K2_GetActorLocation` (`GameplayStatics.GetPlayerPawn` 0))))))

(fn `MoveTowardsPlayer`
  (`self.AddMovementInput` (`KismetMathLibrary.GetForwardVector` (`self.K2_GetActorRotation`))))

(fn `PlayerIsInDistance`
  (returns (IsInDistance :type Boolean))
  (bind _distance (`self.GetDistanceBetweenPlayer`))
  (return (<= _distance 10000.0)))

(fn `PlayerIsToClose`
  (returns (IsInDistance :type Boolean))
  (bind _distance (`self.GetDistanceBetweenPlayer`))
  (return (not (>= _distance 1500.0))))

(fn `RotateTowardsPlayer`
  (params (InterpTime :type "Float (double-precision)") (Delta :type "Float (double-precision)"))
  (`self.SetActorRotation` (`KismetMathLibrary.RInterpTo` (`self.K2_GetActorRotation`) (`KismetMathLibrary.FindLookAtRotation` (`self.K2_GetActorLocation`) (`self.K2_GetActorLocation` (`GameplayStatics.GetPlayerPawn` 0))) Delta InterpTime)))

(fn `UserConstructionScript`)