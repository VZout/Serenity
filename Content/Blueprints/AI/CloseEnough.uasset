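; CloseEnough is a behavior tree decorator for enemy AI that gates a branch on distance to the followed target.
; It casts its owner to AIC_Enemy and measures from the controlled pawn to the TargetToFollow blackboard actor.
; Despite its name, it passes when that distance is at or beyond AcceptableDistance, and it prints a leftover debug string on each check.
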(fn `PerformConditionCheck`
  (params (OwnerActor :type "Actor Object Reference"))
  (returns (ReturnValue :type Boolean))
  (bind _asaic_enemy (cast `/Game/Blueprints/AI/AIC_Enemy` OwnerActor))
  (set `self.AIC_Ref` _asaic_enemy)
  (`KismetSystemLibrary.PrintString` "boyoboy")
  (return (>= (`KismetMathLibrary.VSize` (- (`Actor.K2_GetActorLocation` (`BTFunctionLibrary.GetBlackboardValueAsActor` (`self.TargetToFollow`))) (`Actor.K2_GetActorLocation` (`Controller.K2_GetPawn` (`self.AIC_Ref`))))) (`self.AcceptableDistance`))))