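; Behavior tree aggro check that looks for targets around an AIC_Enemy's pawn on each tick and writes them to the blackboard.
; It caches the controller, sphere-traces nearby objects of the desired types, then line-traces to each on the Camera channel, ignoring all PlayerShip actors.
; A matching hit sets TargetToFollow and TargetLocation, while a mismatch clears only TargetToFollow, so later results overwrite earlier ones.
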(event `self.ReceiveTick`
  (params (OwnerActor :type "Actor Object Reference") (DeltaSeconds :type "Float (single-precision)"))
  (bind _returnvalue (`Actor.K2_GetActorLocation` (`Controller.K2_GetPawn` (`self.OBJ Ref`))))
  (if (not (!= (`self.OBJ Ref`) null))
    (bind _asaic_enemy (cast `/Game/Blueprints/AI/AIC_Enemy` OwnerActor))
    (set `self.OBJ Ref` _asaic_enemy))
  (bind _outactors (`GameplayStatics.GetAllActorsOfClass` "/Script/Serenity.PlayerShip"))
  (`KismetSystemLibrary.PrintString` "AllActorsOfClkassComplete")
  (set `self.MyLocation` _returnvalue)
  (bind _outhits (`KismetSystemLibrary.SphereTraceMultiForObjects` _returnvalue (- _returnvalue (0.0 0.0 0.0)) 1500.0 (`self.DesiredObjectTypes`)))
  (for _array_element _outhits
    (bind (_bblockinghit _binitialoverlap _time _location _impactpoint _normal _impactnormal _physmat _hitactor) (`GameplayStatics.BreakHitResult` _array_element))
    (bind _outhit (`KismetSystemLibrary.LineTraceSingle` (`self.MyLocation`) (`Actor.K2_GetActorLocation` _hitactor) "TraceTypeQuery2" false _outactors))
    (bind (_bblockinghit_2 _binitialoverlap_2 _time_2 _location_2 _impactpoint_2 _normal_2 _impactnormal_2 _physmat_2 _hitactor_2) (`GameplayStatics.BreakHitResult` _outhit))
    (if (== _hitactor_2 _hitactor)
      (`KismetSystemLibrary.PrintString` "Trace returnd true")
      (`BTFunctionLibrary.SetBlackboardValueAsObject` (`self.TargetToFollow`) _hitactor_2)
      (`BTFunctionLibrary.SetBlackboardValueAsVector` (`self.TargetLocation`) (`Actor.K2_GetActorLocation` _hitactor_2))
      (else
        (`KismetSystemLibrary.PrintString` "tracereturnedfalse")
        (`BTFunctionLibrary.SetBlackboardValueAsObject` (`self.TargetToFollow`))))))