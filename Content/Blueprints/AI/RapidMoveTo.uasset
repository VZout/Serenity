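; RapidMoveTo is a Behavior Tree task that sends an enemy AI's pawn toward the blackboard TargetToFollow actor.
; It caches the AIC_Enemy controller on first execution, then issues an AIMoveTo with a wide acceptance radius.
; The immediate Then pin prints a debug string and finishes the task as failed without awaiting the move result.
; A failed controller cast leaves the task unfinished.
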(event `self.ReceiveExecute`
  (params (OwnerActor :type "Actor Object Reference"))
  (if (not (!= (`self.AIC_Ref`) null))
    (bind _asaic_enemy (cast `/Game/Blueprints/AI/AIC_Enemy` OwnerActor))
    (set `self.AIC_Ref` _asaic_enemy))
  (`|AIMoveTo` (`Controller.K2_GetPawn` (`self.AIC_Ref`)) (0.0 0.0 0.0) (`BTFunctionLibrary.GetBlackboardValueAsActor` (`self.TargetToFollow`)) 500.0
    (:`then`
      (`KismetSystemLibrary.PrintString` "Hello")
      (`self.FinishExecute` false))))